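; Base character Blueprint that handles the sniper scope overlay and an Escape-to-quit key.
; ShowSniperScopeWidget lazily creates and caches the scope widget, adds it to the viewport, then plays its zoom animation forward or in reverse with matching 2D sounds.
; BeginPlay, Tick and the construction script are empty.
; Disconnected leftovers cover overhead net-role display, session create/join calls and debug spheres.
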(event `self.ShowSniperScopeWidget`
  (params (bShowScope :type Boolean))
  (bind _snperscopewidget (`self.SnperScopeWidget`))
  (bind _snperscopewidget_2 (`self.SnperScopeWidget`))
  (`/Engine/EditorBlueprintResources/StandardMacros.IsValid` (`self.SnperScopeWidget`)
    (:`Is Valid`
      _)
    (:`Is Not Valid`
      (bind _returnvalue (`|CreateWidget` "/Game/BP/HUD/WB_SniperScope.WB_SniperScope_C"))
      (bind _output_get (set `self.SnperScopeWidget` _returnvalue))
      (`UserWidget.AddToViewport` _output_get 0)))
  (if bShowScope
    (`/Engine/EditorBlueprintResources/StandardMacros.IsValid` _snperscopewidget_2
      (:`Is Valid`
        (`UserWidget.PlayAnimation` _snperscopewidget_2 (`/Game/BP/HUD/WB_SniperScope.ScopeZoomIn` _snperscopewidget_2) 0.0 1 "Forward" 1.0 false)
        (`GameplayStatics.PlaySound2D` "/Game/Assets/MilitaryWeapSilver/Sound/SniperRifle/Cues/SniperRifle_ZoomIn_Cue.SniperRifle_ZoomIn_Cue" 1.0 1.0 0.0 null null)))
    (else
      (`/Engine/EditorBlueprintResources/StandardMacros.IsValid` _snperscopewidget
        (:`Is Valid`
          (`UserWidget.PlayAnimation` _snperscopewidget (`/Game/BP/HUD/WB_SniperScope.ScopeZoomIn` _snperscopewidget) 0.0 1 "Reverse" 1.0 false)
          (`GameplayStatics.PlaySound2D` "/Game/Assets/MilitaryWeapSilver/Sound/SniperRifle/Cues/SniperRifle_ZoomOut_Cue.SniperRifle_ZoomOut_Cue" 1.0 1.0 0.0 null null))))))

(event `self.ReceiveBeginPlay`)

(event `self.ReceiveTick`
  (params (DeltaSeconds :type "Float (single-precision)")))

(event `Key|Escape`
  (params (Key :type "Key Structure"))
  (:`Pressed`
    (`KismetSystemLibrary.QuitGame` null "Quit")))

(event `Key|One`
  (params (Key :type "Key Structure"))
  ;[1 1 1] Menu를 사용하므로 더 이상 사용하지 않음.
)

(event `Key|Two`
  (params (Key :type "Key Structure"))
  ;[1 1 1] Menu를 사용하므로 더 이상 사용하지 않음.
)

(fn `UserConstructionScript`)